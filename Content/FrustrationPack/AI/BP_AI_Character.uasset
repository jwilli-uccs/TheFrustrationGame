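; AI character that models the player's Autonomy, Competence and Relatedness frustration as meters clamped between zero and one.
; Looping named timers charge or drain each meter by its frustrated flag, and a charge timer clears at full.
; Player character dispatchers force Competence frustration, select the frustration method and report key presses.
; Tick passes method and key to the AI controller's Blackboard, while BeginPlay adds an AI HUD and FPS display.
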(event `self.ReceiveBeginPlay`
  ; Draw AIHUD on screen
  (bind _returnvalue (`|CreateWidget` "/Game/FrustrationPack/UI/AIHUD.AIHUD_C"))
  (`UserWidget.AddToViewport` _returnvalue 0)
  (`KismetSystemLibrary.ExecuteConsoleCommand` "stat fps" null) ; Display FPS
  ; Listen for Forced Frustration Event from Player Character
  (bind _asbp_third_person_character (cast `/Game/ThirdPerson/Blueprints/BP_ThirdPersonCharacter` (`GameplayStatics.GetPlayerCharacter` 0)))
  (bind _output_get (set `self.As BP Third Person Character` _asbp_third_person_character))
  (add `/Game/ThirdPerson/Blueprints/BP_ThirdPersonCharacter.ForcedFrustrationEvent` _output_get (delegate `ForcedFrustration`))
  ; Listen for SelectFrustration0 Event from Player Character
  (bind _asbp_third_person_character_2 (cast `/Game/ThirdPerson/Blueprints/BP_ThirdPersonCharacter` (`GameplayStatics.GetPlayerCharacter` 0)))
  (bind _output_get_2 (set `self.As BP Third Person Character` _asbp_third_person_character_2))
  (add `/Game/ThirdPerson/Blueprints/BP_ThirdPersonCharacter.SelectFrustrationMethod0Event` _output_get_2 (delegate `FrustrationMethod0`))
  ; Listen for SelectFrustration1 Event from Player Character
  (bind _asbp_third_person_character_3 (cast `/Game/ThirdPerson/Blueprints/BP_ThirdPersonCharacter` (`GameplayStatics.GetPlayerCharacter` 0)))
  (bind _output_get_3 (set `self.As BP Third Person Character` _asbp_third_person_character_3))
  (add `/Game/ThirdPerson/Blueprints/BP_ThirdPersonCharacter.SelectFrustrationMethod1Event` _output_get_3 (delegate `SelectFrustrationMethod1`))
  ; Listen for SelectFrustration2 Event from Player Character
  (bind _asbp_third_person_character_4 (cast `/Game/ThirdPerson/Blueprints/BP_ThirdPersonCharacter` (`GameplayStatics.GetPlayerCharacter` 0)))
  (bind _output_get_4 (set `self.As BP Third Person Character` _asbp_third_person_character_4))
  (add `/Game/ThirdPerson/Blueprints/BP_ThirdPersonCharacter.SelectFrustrationMethod2Event` _output_get_4 (delegate `SelectFrustrationMethod2`))
  ; Listen for AnyKey Event from Player Character
  (bind _asbp_third_person_character_5 (cast `/Game/ThirdPerson/Blueprints/BP_ThirdPersonCharacter` (`GameplayStatics.GetPlayerCharacter` 0)))
  (bind _output_get_5 (set `self.As BP Third Person Character` _asbp_third_person_character_5))
  (add `/Game/ThirdPerson/Blueprints/BP_ThirdPersonCharacter.AnyKeyEvent` _output_get_5 (delegate `AnyKeyEvent`)))

(event `SelectFrustrationMethod2`
  ; Listen for SelectFrustration2 Event from Player Character
  (set `self.FrustrationMethod` "NewEnumerator2"))

(event `AnyKeyEvent`
  ; Listen for AnyKey Event from Player Character
  (bind _asbp_third_person_character (cast `/Game/ThirdPerson/Blueprints/BP_ThirdPersonCharacter` (`GameplayStatics.GetPlayerCharacter` 0)))
  (set `self.KeyPressed` (`/Game/ThirdPerson/Blueprints/BP_ThirdPersonCharacter.KeyPressed` _asbp_third_person_character)))

(event `FrustrationMethod0`
  ; Listen for SelectFrustration0 Event from Player Character
  (set `self.FrustrationMethod` "NewEnumerator0"))

(event `SelectFrustrationMethod1`
  ; Listen for SelectFrustration1 Event from Player Character
  (set `self.FrustrationMethod` "NewEnumerator1"))

(event `ForcedFrustration`
  (params (Pressed :type Boolean))
  ; Listen for Forced Frustration Event from Player Character
  (if Pressed
    (`self.StartFrustration` "NewEnumerator1")
    (else
      (`self.StopFrustration` "NewEnumerator1"))))

(event `self.ReceiveTick`
  (params (DeltaSeconds :type "Float (single-precision)"))
  ; Update Blackboard
  (`/Game/FrustrationPack/AI/BP_AIController.UpdateBlackboard` (`self.theAIController`) (`self.FrustrationMethod`) (`self.KeyPressed`)))

(event `StartFrustrationC`
  (`self.StartFrustration` "NewEnumerator1"))

(event `EndFrustrationC`
  (`self.StopFrustration` "NewEnumerator1"))

(event `StartFrustrationA`
  (`self.StartFrustration` "NewEnumerator0"))

(event `ManageFrustrationA`
  ; Manage Frustration Charge and Drain
  ;; Manage Frustration Charge and Drain Autonomy
  (if (`self.IsFrustratedA`)
    (`self.ManageFrustrationCharge` "NewEnumerator0")
    (else
      (`self.ManageFrustrationDrain` "NewEnumerator0"))))

(event `EndFrustrationA`
  (`self.StopFrustration` "NewEnumerator0"))

(event `ManageFrustrationC`
  ; Manage Frustration Charge and Drain
  ;; Manage Frustration Charge and Drain Competence
  (if (`self.IsFrustratedC`)
    (`self.ManageFrustrationCharge` "NewEnumerator1")
    (else
      (`self.ManageFrustrationDrain` "NewEnumerator1"))))

(event `ManageFrustrationR`
  ; Manage Frustration Charge and Drain
  ;; Manage Frustration Charge and Drain Relatedness
  (if (`self.IsFrustratedR`)
    (`self.ManageFrustrationCharge` "NewEnumerator2")
    (else
      (`self.ManageFrustrationDrain` "NewEnumerator2"))))

(fn `UserConstructionScript`
  (`parent.UserConstructionScript`))